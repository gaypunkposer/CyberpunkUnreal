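; Game mode that runs conversations between the player and another participant, in active or timed passive form.
; It caches the player pawn on BeginPlay, holds a dialogue context and pushes speaker names, lines and options to the player's HUD.
; Selection works in two steps, revealing options and then choosing one, with a progress shortcut for single-option nodes.
; The dialogue closes when choosing a child fails.
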(event `self.ReceiveBeginPlay`
  (bind _asbp_player (cast `/Game/PlayerCharacter/Blueprints/BP_Player` (`GameplayStatics.GetPlayerPawn` 0)))
  (set `self.Player` _asbp_player))

(event `self.ReceiveTick`
  (params (DeltaSeconds :type "Float (single-precision)")))

(fn `Begin Active Dialogue`
  (params (`Dialogue Object` :type "DlgDialogue Object Reference") (`Other Participant` :type "Actor Object Reference"))
  (bind _returnvalue (`DlgManager.StartDialogue2` `Dialogue Object` (`GameplayStatics.GetPlayerPawn` 0) `Other Participant`))
  (set `self.DialogueContext` _returnvalue)
  (`/Game/PlayerCharacter/Blueprints/BP_PlayerHUDWidget.EnableDialogue` (`/Game/PlayerCharacter/Blueprints/BP_Player.HUD` (`self.Player`)) true 0.0)
  (`self.Update Dialogue`))

(fn `Begin Passive Dialogue`
  (params (`Dialogue Object` :type "DlgDialogue Object Reference") (`Other Participant` :type "Actor Object Reference") (`Dialogue Shown Time` :type "Float (double-precision)"))
  (bind _returnvalue (`DlgManager.StartDialogue2` `Dialogue Object` (`GameplayStatics.GetPlayerPawn` 0) `Other Participant`))
  (set `self.DialogueContext` _returnvalue)
  (`/Game/PlayerCharacter/Blueprints/BP_PlayerHUDWidget.EnableDialogue` (`/Game/PlayerCharacter/Blueprints/BP_Player.HUD` (`self.Player`)) false `Dialogue Shown Time`)
  (`self.Update Dialogue`))

(fn `Disable Dialogue`
  (set `self.DialogueContext` null)
  (`/Game/PlayerCharacter/Blueprints/BP_PlayerHUDWidget.DisableDialogue` (`/Game/PlayerCharacter/Blueprints/BP_Player.HUD` (`self.Player`)))
  (set `self.Dialogue Active` false))

(fn `Progress Dialogue`
  (bind _dialoguecontext (`self.DialogueContext`))
  (`/Engine/EditorBlueprintResources/StandardMacros.IsValid` _dialoguecontext
    (:`Is Valid`
      (if (== (`DlgContext.GetOptionNum` _dialoguecontext) 1)
        (if (`self.Showing Options`)
          (bind _returnvalue (`DlgContext.ChooseChild` _dialoguecontext 0))
          (set `self.Showing Options` false)
          (if (not _returnvalue)
            (`self.Disable Dialogue`)
            (else
              (`self.Update Dialogue`)))
          (else
            (`self.Show Options`)))))))

(fn `Select Option`
  (params (Selected :type Integer))
  (bind _dialoguecontext (`self.DialogueContext`))
  (`/Engine/EditorBlueprintResources/StandardMacros.IsValid` _dialoguecontext
    (:`Is Valid`
      (if (`self.Showing Options`)
        (if (< Selected (`DlgContext.GetOptionNum` _dialoguecontext))
          (bind _returnvalue (`DlgContext.ChooseChild` _dialoguecontext Selected))
          (set `self.Showing Options` false)
          (if _returnvalue
            (`self.Update Dialogue`)
            (else
              (`self.Disable Dialogue`))))
        (else
          (`self.Show Options`))))))

(fn `Show Options`
  (bind _dialoguecontext (`self.DialogueContext`))
  (`/Engine/EditorBlueprintResources/StandardMacros.IsValid` _dialoguecontext
    (:`Is Valid`
      (`KismetArrayLibrary.Array_Clear` (`self.Options`))
      (for _index (range (`DlgContext.GetOptionNum` _dialoguecontext))
        (`KismetArrayLibrary.Array_Add` (`self.Options`) (`DlgContext.GetOptionText` _dialoguecontext _index)))
      (set `self.Showing Options` true)
      (`/Game/PlayerCharacter/Blueprints/BP_ActiveDialogueWidget.SetDialogueOptions` (`/Game/PlayerCharacter/Blueprints/BP_PlayerHUDWidget.ActiveDialogue` (`/Game/PlayerCharacter/Blueprints/BP_Player.HUD` (`self.Player`))) (`self.Options`)))))

(fn `Update Dialogue`
  (bind _dialoguecontext (`self.DialogueContext`))
  (`/Engine/EditorBlueprintResources/StandardMacros.IsValid` _dialoguecontext
    (:`Is Valid`
      (set `self.Showing Options` false)
      (`/Game/PlayerCharacter/Blueprints/BP_PlayerHUDWidget.UpdateDialogue` (`/Game/PlayerCharacter/Blueprints/BP_Player.HUD` (`self.Player`)) (`DlgContext.GetActiveNodeParticipantName` _dialoguecontext) (`DlgContext.GetActiveNodeText` _dialoguecontext)))))

(fn `UserConstructionScript`)