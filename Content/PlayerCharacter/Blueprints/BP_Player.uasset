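; BP_Player is the player character Blueprint, handling startup references and pushing of physical objects.
; On BeginPlay it caches the body mesh's BP_Anim_woman instance as the viewmodel animation instance and stores the CyberpunkGameMode.
; Capsule hits are meant to push Movable components with an impulse equal to movement velocity.
; That push requires HitComponent to differ from the capsule, which this capsule-bound event normally never satisfies.
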(event `self.ReceiveBeginPlay`
  (`|ExecutionSequence`
    (:`then_0`
      (bind _asbp_anim_woman (cast `/Game/PlayerCharacter/Blueprints/BP_Anim_woman` (`SkeletalMeshComponent.GetAnimInstance` (`self.BodyMesh`))))
      (set `self.Viewmodel Anim Instance` _asbp_anim_woman))
    (:`then_1`
      (bind _ascyberpunk_game_mode (cast `CyberpunkGameMode` (`GameplayStatics.GetGameMode`)))
      (set `self.Gamemode` _ascyberpunk_game_mode))))

(event `self.CapsuleCollider.OnComponentHit`
  (params (HitComponent :type "PrimitiveComponent Object Reference") (OtherActor :type "Actor Object Reference") (OtherComp :type "PrimitiveComponent Object Reference") (NormalImpulse :type "Vector Structure") (Hit :type "HitResult Structure (by ref)"))
  (if (and (!= HitComponent (`self.CapsuleCollider`)) (`|EnumEquality` (`SceneComponent.Mobility` OtherComp) "Movable"))
    (`PrimitiveComponent.AddImpulse` OtherComp (`MovementComponent.Velocity` (`self.MovementComponent`)) "None" false)))

(fn `UserConstructionScript`)